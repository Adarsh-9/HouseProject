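; TVScreenBP is a TV screen actor that cycles through four video channels.
; On BeginPlay it opens a separate media source on each of four media players: an intro, a project demo, Tank Battle and Excape The Room.
; ChangeChannel applies the current index's material to the screen mesh and points the TV sound at the matching player, then increments the index, wrapping by player count.
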(event Custom|ChangeChannel
  (bind _mediaplayer (Variables|Default|GetMediaPlayer))
  (bind _currentindex (Variables|Default|GetCurrentIndex))
  (bind _returnvalue (Utilities|Array|Length _mediaplayer))
  (bind _returnvalue_2 (Math|Integer|%(Integer) _currentindex _returnvalue))
  (Rendering|Material|SetMaterial (Variables|Debug|GetStaticMeshComponent) 0 (Utilities|Array|Get(acopy) (Variables|Default|GetMaterials) _returnvalue_2))
  (Media|MediaSoundComponent|SetMediaPlayer (Variables|Default|GetTVSound) (Utilities|Array|Get(acopy) (Variables|Default|GetMediaPlayer) _returnvalue_2))
  (Math|Integer|IncrementInt (Variables|Default|GetCurrentIndex)))

(event EventBeginPlay
  (Media|MediaPlayer|OpenSource (Utilities|Array|Get(acopy) (Variables|Default|GetMediaPlayer)) "/Game/Movies/Videos/Intro.Intro")
  (Media|MediaPlayer|OpenSource (Utilities|Array|Get(acopy) (Variables|Default|GetMediaPlayer) 1) "/Game/Movies/Videos/ProjectDemo.ProjectDemo")
  (Media|MediaPlayer|OpenSource (Utilities|Array|Get(acopy) (Variables|Default|GetMediaPlayer) 2) "/Game/Movies/Videos/TankBattle.TankBattle")
  (Media|MediaPlayer|OpenSource (Utilities|Array|Get(acopy) (Variables|Default|GetMediaPlayer) 3) "/Game/Movies/Videos/ExcapeTheRoom.ExcapeTheRoom"))

(event Collision|EventActorBeginOverlap
  (params (OtherActor :type Actor%20Object%20Reference)))

(event EventTick
  (params (DeltaSeconds :type Float%20%28single-precision%29)))

(fn ConstructionScript)