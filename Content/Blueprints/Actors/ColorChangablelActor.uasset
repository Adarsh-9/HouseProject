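; Actor whose world-space prompt widget shows the name of the item, presumably one with customizable color or style.
; On BeginPlay it casts the PromptWidget component's user widget to Prompt and sets its NameOfItem from the StyleCustomization data.
; Overlap and Tick events are empty, and the construction script does nothing.
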(event EventBeginPlay
  (bind _asprompt (Utilities|Casting|CastToPrompt (UserInterface|GetUserWidgetObject (Variables|Default|GetPromptWidget))))
  (Variables|/Game/Blueprints/UMG/Prompt.Prompt_C|SetNameOfItem _asprompt (Utilities|Text|ToText(Name) (Variables|/Script/WallColorPicker.StyleCustomizationComponent|GetNameOfItem (Variables|Default|GetStyleCustomization)))))

(event Collision|EventActorBeginOverlap
  (params (OtherActor :type Actor%20Object%20Reference)))

(event EventTick
  (params (DeltaSeconds :type Float%20%28single-precision%29)))

(fn ConstructionScript)